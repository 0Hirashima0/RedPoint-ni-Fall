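; BP_Ice is an ice actor that can be collected by the ice character or melted away by damage.
; A capsule overlap with BP_IceChara prints a pickup message and destroys the ice.
; Any damage prints a message, waits briefly, destroys the ice, then spawns a BP_Ice_delete well below it with a movable sphere as the fallen, melted remains.
; Other spawn and cast nodes are disconnected leftovers.
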(event `self.Ice_Sphere.OnComponentBeginOverlap`
  (params (OverlappedComponent :type "PrimitiveComponent Object Reference") (OtherActor :type "Actor Object Reference") (OtherComp :type "PrimitiveComponent Object Reference") (OtherBodyIndex :type Integer) (bFromSweep :type Boolean) (SweepResult :type "HitResult Structure (by ref)")))

(event `self.Capsule.OnComponentBeginOverlap`
  (params (OverlappedComponent :type "PrimitiveComponent Object Reference") (OtherActor :type "Actor Object Reference") (OtherComp :type "PrimitiveComponent Object Reference") (OtherBodyIndex :type Integer) (bFromSweep :type Boolean) (SweepResult :type "HitResult Structure (by ref)"))
  ;[1 1 1] 人間かコーンか、どっちがいいかなぁ？？
  (cast `/Game/IceCatch/BP_IceChara` OtherActor)
  (`KismetSystemLibrary.PrintString` "アイスゲット！")
  (`self.K2_DestroyActor`))

(event `self.ReceiveBeginPlay`)

(event `self.ReceiveAnyDamage`
  (params (Damage :type "Float (single-precision)") (DamageType :type "DamageType Object Reference") (InstigatedBy :type "Controller Object Reference") (DamageCauser :type "Actor Object Reference"))
  (bind _returnvalue_location (`KismetMathLibrary.BreakTransform` (`self.GetTransform`)))
  (`KismetSystemLibrary.PrintString` "アイス「痛い」")
  (`KismetSystemLibrary.Delay` 0.7)
  (`self.K2_DestroyActor`)
  (bind _returnvalue (`|SpawnActorFromClass` "/Game/IceCatch/BP_Ice_delete.BP_Ice_delete_C" (`KismetMathLibrary.Conv_VectorToTransform` (+ _returnvalue_location (0.0 0.0 -1000.0))) "Undefined" "OverrideRootScale" null null)) ; スポーンすｒ
  (`SceneComponent.SetMobility` (`/Game/IceCatch/BP_Ice_delete.Sphere` _returnvalue) "Movable") ; わからん
)

(fn `UserConstructionScript`)