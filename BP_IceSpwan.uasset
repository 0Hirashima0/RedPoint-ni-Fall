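; BP_IceSpwan is a spawner that endlessly drops ice at random spots inside its UnderBox volume, starting at BeginPlay.
; Each drop spawns a BP_Ice_Point marker (the red point) at a random location, then a BP_Ice high above it.
; The cycle alternates a single drop and a pair of drops, separated by Delays, and wires back to the start to repeat.
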(event `self.ReceiveBeginPlay`
  (bind _under_box (`self.Under_Box`))
  (bind _under_box_2 (`self.Under_Box`))
  (for _ (range 1) :!label _label
    (bind _returnvalue (`|SpawnActorFromClass` "/Game/IceCatch/BP_Ice_Point.BP_Ice_Point_C" (`KismetMathLibrary.MakeTransform` (`KismetMathLibrary.RandomPointInBoundingBox` (`SceneComponent.K2_GetComponentLocation` _under_box_2) (`BoxComponent.BoxExtent` _under_box_2))) "Undefined" "OverrideRootScale" null null)) ; 先ず赤ポイントをスポーン
    (bind _returnvalue_location (`KismetMathLibrary.BreakTransform` (`self.GetTransform` (cast `/Game/IceCatch/BP_Ice_Point` _returnvalue :!pure true))))
    (`|SpawnActorFromClass` "/Game/IceCatch/BP_Ice.BP_Ice_C" (`KismetMathLibrary.MakeTransform` (+ _returnvalue_location (0.0 0.0 1000.0))) "Undefined" "OverrideRootScale" null null) ; スポーンする
    (`KismetSystemLibrary.Delay` 7.0)
    (for _ (range 2)
      (bind _returnvalue_2 (`|SpawnActorFromClass` "/Game/IceCatch/BP_Ice_Point.BP_Ice_Point_C" (`KismetMathLibrary.MakeTransform` (`KismetMathLibrary.RandomPointInBoundingBox` (`SceneComponent.K2_GetComponentLocation` _under_box) (`BoxComponent.BoxExtent` _under_box))) "Undefined" "OverrideRootScale" null null))
      (bind _returnvalue_location_2 (`KismetMathLibrary.BreakTransform` (`self.GetTransform` (cast `/Game/IceCatch/BP_Ice_Point` _returnvalue_2 :!pure true))))
      (`|SpawnActorFromClass` "/Game/IceCatch/BP_Ice.BP_Ice_C" (`KismetMathLibrary.MakeTransform` (+ _returnvalue_location_2 (0.0 0.0 1000.0))) "Undefined" "OverrideRootScale" null null)
      (`KismetSystemLibrary.Delay` 3.0)
      (goto _label))))

(fn `UserConstructionScript`)